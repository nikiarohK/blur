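; Lever trigger Blueprint that operates a linked Closed_door when its Pulingthelever event fires.
; A FlipFlop alternates the lever between two pull directions, each using its own timeline to lerp the lever's relative rotation between two angles.
; Both directions cast the Door reference and call the same DoorOpen function before the animation starts.
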(event Custom|Puling%20the%20lever
  (Utilities|FlowControl|FlipFlop
    (:A
      (bind _asclosed_door (Utilities|Casting|CastToClosed_door (Variables|Default|Getdoor)))
      (Default|DoorOpen _asclosed_door)
      (bind _newtrack_0 (Timeline|pull PlayFromStart)
        (:Update
          (Transformation|SetRelativeRotation (Variables|Default|Getlever) (Math|Rotator|Lerp(Rotator) "-50.000000,0.000000,0.000000" "-140.000000,0.000000,0.000000" _newtrack_0) false false))))
    (:B
      (bind _asclosed_door_2 (Utilities|Casting|CastToClosed_door (Variables|Default|Getdoor)))
      (Default|DoorOpen _asclosed_door_2)
      (bind _newtrack_0_2 (Timeline|Timeline PlayFromStart)
        (:Update
          (Transformation|SetRelativeRotation (Variables|Default|Getlever) (Math|Rotator|Lerp(Rotator) "-140.000000,0.000000,0.000000" "-50.000000,0.000000,0.000000" _newtrack_0_2) false false))))))

(fn ConstructionScript)