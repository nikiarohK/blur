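; A carryable item actor: a cube that a first-person character can pick up and release.
; Pickup stores the character and sets IsPicked, which has an empty OnRep, and release clears the flag.
; Each Tick on the authority, a held cube loses collision and physics, shrinks to half its released size and snaps to the character's ItemPlace.
; When not held, it regains collision, physics and its larger scale every Tick.
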(event Custom|picked%20up
  (params (player :type Actor%20Object%20Reference))
  (if (not (Variables|Default|Getis%20picked))
    (bind _asbp_first_person_character (Utilities|Casting|CastToBP_FirstPersonCharacter player))
    (Variables|Default|Setis%20picked true)))

(event Custom|released
  (Variables|Default|Setis%20picked false))

(event Custom|own
  (Collision|SetCollisionEnabled (Variables|Default|GetCube) "NoCollision")
  (Physics|SetSimulatePhysics (Variables|Default|GetCube) false)
  (Transformation|SetWorldScale3D (Variables|Default|GetCube) "0.250000,0.250000,0.250000"))

(event Custom|own2
  (Collision|SetCollisionEnabled (Variables|Default|GetCube) "QueryAndPhysics")
  (Physics|SetSimulatePhysics (Variables|Default|GetCube) true)
  (Transformation|SetWorldScale3D (Variables|Default|GetCube) "0.500000,0.500000,0.500000"))

(event EventTick
  (params (DeltaSeconds :type Float%20%28single-precision%29))
  (Networking|SwitchHasAuthority
    (:Authority
      (if (Variables|Default|Getis%20picked)
        (CallFunction|Own)
        (Transformation|SetWorldLocationAndRotation (Variables|Default|GetCube) (Transformation|GetWorldLocation (Variables|/Game/FirstPerson/Blueprints/BP_FirstPersonCharacter.BP_FirstPersonCharacter_C|Getitem%20place (stale Custom|picked%20up _asbp_first_person_character))) (Transformation|GetWorldRotation (Variables|/Game/FirstPerson/Blueprints/BP_FirstPersonCharacter.BP_FirstPersonCharacter_C|Getitem%20place (stale Custom|picked%20up _asbp_first_person_character))) false false)
        (else
          (CallFunction|Own2))))))

(fn ConstructionScript)

(fn OnRepIsPicked)