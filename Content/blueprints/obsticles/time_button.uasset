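; A timed pressure button Blueprint that operates a linked Closed_door when something overlaps its sphere.
; Overlap start plays a timeline that lowers the Rr component, then calls DoorOpen on the door and sets IsOpen.
; Overlap end, if IsOpen, waits for the Timer delay, calls DoorOpen again, and raises the button with a second timeline that clears IsOpen as it updates.
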(event OnComponentBeginOverlap(Sphere)
  (params (OverlappedComponent :type Primitive%20Component%20Object%20Reference) (OtherActor :type Actor%20Object%20Reference) (OtherComp :type Primitive%20Component%20Object%20Reference) (OtherBodyIndex :type Integer) (bFromSweep :type Boolean) (SweepResult :type Hit%20Result%20Structure%20%28by%20ref%29))
  (if (not (Variables|Default|Getis%20open))
    (bind _newtrack_0 (Timeline|Timeline PlayFromStart)
      (:Update
        (Transformation|SetRelativeTransform (Variables|Default|Getrr) (Math|Transform|Lerp(Transform) (Math|Transform|MakeTransform "0, 0, 0" "0, 0, 0" "1.000000,1.000000,0.250000") (Math|Transform|MakeTransform "0.000000,0.000000,-15.000000" "0, 0, 0" "1.000000,1.000000,0.250000") _newtrack_0) false false))
      (:Finished
        (bind _asclosed_door (Utilities|Casting|CastToClosed_door (Variables|Default|Getdoor)))
        (Default|DoorOpen _asclosed_door)
        (Variables|Default|Setis%20open true)))))

(event OnComponentEndOverlap(Sphere)
  (params (OverlappedComponent :type Primitive%20Component%20Object%20Reference) (OtherActor :type Actor%20Object%20Reference) (OtherComp :type Primitive%20Component%20Object%20Reference) (OtherBodyIndex :type Integer))
  (if (Variables|Default|Getis%20open)
    (Utilities|FlowControl|Delay (Variables|Default|Gettimer))
    (bind _asclosed_door (Utilities|Casting|CastToClosed_door (Variables|Default|Getdoor)))
    (Default|DoorOpen _asclosed_door)
    (bind _newtrack_0 (Timeline|Timeline_0 PlayFromStart)
      (:Update
        (Transformation|SetRelativeTransform (Variables|Default|Getrr) (Math|Transform|Lerp(Transform) (Math|Transform|MakeTransform "0.000000,0.000000,-15.000000" "0, 0, 0" "1.000000,1.000000,0.250000") (Math|Transform|MakeTransform "0.000000,0.000000,0.000000" "0, 0, 0" "1.000000,1.000000,0.250000") _newtrack_0) false false)
        (Variables|Default|Setis%20open false)))))

(fn ConstructionScript)