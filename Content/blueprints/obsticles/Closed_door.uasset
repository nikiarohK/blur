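; Door obstacle that toggles between closed and open each time its Dooropen event is called; nothing in this Blueprint calls that event.
; A FlipFlop alternates between two timelines, one for opening and one for closing, each played from the start.
; Each timeline lerps the Cube's relative transform between hardcoded poses, pairing a 90-degree rotation with an offset to mimic a hinged swing, without sweep.
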(event Custom|Door%20open
  (Utilities|FlowControl|FlipFlop
    (:A
      (bind _newtrack_0 (Timeline|Timeline_0 PlayFromStart)
        (:Update
          (Transformation|SetRelativeTransform (Variables|Default|GetCube) (Math|Transform|Lerp(Transform) (Math|Transform|MakeTransform "0.000000,0.000000,100.000000" "0, 0, 0" "0.050000,1.000000,2.000000") (Math|Transform|MakeTransform "-42.500000,-43.000000,100.000000" "0.000000,90.000000,0.000000" "0.050000,1.000000,2.000000") _newtrack_0) false false))))
    (:B
      (bind _newtrack_0_2 (Timeline|Timeline PlayFromStart)
        (:Update
          (Transformation|SetRelativeTransform (Variables|Default|GetCube) (Math|Transform|Lerp(Transform) (Math|Transform|MakeTransform "-42.500000,-43.000000,100.000000" "0.000000,90.000000,0.000000" "0.050000,1.000000,2.000000") (Math|Transform|MakeTransform "0.000000,0.000000,100.000000" "0, 0, 0" "0.050000,1.000000,2.000000") _newtrack_0_2) false false))))))

(fn ConstructionScript)